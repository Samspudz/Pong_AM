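; BP_Invisiball2 is an invisible companion actor to BP_Ball that removes itself once it travels out of bounds along the X axis.
; It hides its Sphere on BeginPlay and checks that sphere's world X position every Tick against symmetric limits.
; Past either limit it destroys itself, then finds BP_Ball by class and clears its InvisiBallExists flag.
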(event `self.ReceiveBeginPlay`
  (`SceneComponent.SetVisibility` (`self.Sphere`) false false))

(event `self.ReceiveTick`
  (params (DeltaSeconds :type "Float (single-precision)"))
  (bind _returnvalue_x (`KismetMathLibrary.BreakVector` (`SceneComponent.K2_GetComponentLocation` (`self.Sphere`))))
  (if (<= _returnvalue_x -1400.0)
    (`self.K2_DestroyActor` :!label _label)
    (bind _returnvalue (`GameplayStatics.GetActorOfClass` "/Game/BP_Ball.BP_Ball_C"))
    (set `/Game/BP_Ball.InvisiBallExists` false _returnvalue)
    (elif (>= _returnvalue_x 1400.0)
      (goto _label))))

(fn `UserConstructionScript`)