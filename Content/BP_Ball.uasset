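; BP_Ball is a physics ball that launches along negative X on BeginPlay and speeds up with every hit.
; BallSpeedUp raises BallSpeed, clamps the sphere's velocity magnitude to exactly that value and prints the velocity.
; Hits also spawn a BP_InvisiBall at the ball's transform when InvisiBallExists is already true.
; Each Tick checks both X bounds; leaving them makes BP_BallSpawner spawn a replacement and destroys this ball.
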(event `self.ReceiveBeginPlay`
  (`PrimitiveComponent.AddImpulse` (`self.Sphere`) (-1000.0 0.0 0.0) "None" true))

(event `self.ReceiveTick`
  (params (DeltaSeconds :type "Float (single-precision)"))
  (`self.BallRespawn`))

(event `self.ReceiveHit`
  (params (MyComp :type "PrimitiveComponent Object Reference") (Other :type "Actor Object Reference") (OtherComp :type "PrimitiveComponent Object Reference") (bSelfMoved :type Boolean) (HitLocation :type "Vector Structure") (HitNormal :type "Vector Structure") (NormalImpulse :type "Vector Structure") (Hit :type "HitResult Structure (by ref)"))
  (`self.BallSpeedUp`)
  (if (`self.InvisiBallExists`)
    (`|SpawnActorFromClass` "/Game/BP_InvisiBall.BP_InvisiBall_C" (`self.GetTransform`) "Undefined" "MultiplyWithRoot" null null)
    (set `self.InvisiBallExists` true)))

(fn `BallRespawn`
  (bind _returnvalue_x (`KismetMathLibrary.BreakVector` (`SceneComponent.K2_GetComponentLocation` (`self.Sphere`))))
  (if (<= _returnvalue_x -1600.0)
    (bind _returnvalue (`GameplayStatics.GetActorOfClass` "/Game/BP_BallSpawner.BP_BallSpawner_C" :!label _label))
    (`/Game/BP_BallSpawner.SpawnBall` _returnvalue)
    (`self.K2_DestroyActor`)
    (elif (>= _returnvalue_x 1600.0)
      (goto _label))))

(fn `BallSpeedUp`
  (bind _ballspeed (`self.BallSpeed`))
  (bind _sphere (`self.Sphere`))
  (set `self.BallSpeed` (+ (`self.BallSpeed`) 20.0))
  (bind _returnvalue (`PrimitiveComponent.GetPhysicsLinearVelocity` _sphere "None"))
  (`PrimitiveComponent.SetPhysicsLinearVelocity` _sphere (`KismetMathLibrary.ClampVectorSize` _returnvalue _ballspeed _ballspeed) false "None")
  (bind _returnvalue_2 (`PrimitiveComponent.GetPhysicsLinearVelocity` (`self.Sphere`) "None"))
  (`KismetSystemLibrary.PrintString` (`KismetStringLibrary.Conv_VectorToString` _returnvalue_2) true true (struct :`G` 1.0 :`B` 0.161651 :`A` 1.0)))

(fn `UserConstructionScript`)