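; BP_CPUPaddle is a computer-controlled paddle that follows the height of the ball.
; Every Tick it looks up BP_Ball with GetActorOfClass and, after checking the result, calls MoveComponentTo on its Cube.
; The move targets a fixed relative X and the ball's world Z, with MoveTime setting the move's duration.
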(event `self.ReceiveTick`
  (params (DeltaSeconds :type "Float (single-precision)"))
  (`parent.ReceiveTick` DeltaSeconds)
  (bind _returnvalue (`GameplayStatics.GetActorOfClass` "/Game/BP_Ball.BP_Ball_C"))
  (if (!= _returnvalue null)
    (bind (_returnvalue_x _returnvalue_y _returnvalue_z) (`KismetMathLibrary.BreakVector` (`self.K2_GetActorLocation` _returnvalue)))
    (`KismetSystemLibrary.MoveComponentTo` (`self.Cube`) (`KismetMathLibrary.MakeVector` 1350.0 0.0 _returnvalue_z) (struct) false false (`self.MoveTime`))))

(fn `UserConstructionScript`
  (`parent.UserConstructionScript`))